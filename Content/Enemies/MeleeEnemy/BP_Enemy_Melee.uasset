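; Melee enemy Blueprint that gives its parent enemy class sword-style attacks, a block reaction and weapon handling.
; Attack events pass a target, montage and damage to BPCAttacks for ground smash, short-range, long-range and spinning attacks, scaling damage by the game instance's Tuyosa value.
; Montage notifies spawn a fork weapon on the hand socket or destroy it, and it reports ideal attack and defend ranges.
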(event `self.ReceiveBeginPlay`
  (`parent.ReceiveBeginPlay`)
  (`/Game/DamageSystem/W_HealthBar.Color` (`self.Health`) (`self.Color`)))

(event `GroundSmashAttack`
  (params (AttackTarget :type "Actor Object Reference"))
  ;[1 1 1] Attacks
  (bind _new_atk (`self.ATK` 5.0))
  (`/Game/Attacks/BPC_Attacks.GroundSmash` (`self.BPC_Attacks`) (make `/Game/Attacks/S_AttackInfo` AttackTarget "/Game/Enemies/Soseji2/Animation/Montage_Melee_GroundSmash.Montage_Melee_GroundSmash" (make `/Game/DamageSystem/S_DamageInfo` _new_atk "NewEnumerator3")) 300.0))

(event `ShortRangeAttack`
  (params (AttackTarget :type "Actor Object Reference"))
  ;[1 1 1] Attacks
  (bind _new_atk (`self.ATK` 2.0))
  (`/Game/Attacks/BPC_Attacks.PrimaryMeleeAttack` (`self.BPC_Attacks`) (make `/Game/Attacks/S_AttackInfo` AttackTarget "/Game/Enemies/Soseji2/Animation/Montage_Sword_Slash.Montage_Sword_Slash" (make `/Game/DamageSystem/S_DamageInfo` _new_atk "NewEnumerator1" "NewEnumerator0" false true true)) 20.0 200.0))

(event `LongRangeAttack`
  (params (AttackTarget :type "Actor Object Reference"))
  ;[1 1 1] Attacks
  (bind _new_atk (`self.ATK` 2.0))
  (`/Game/Attacks/BPC_Attacks.LongRangeMeleeAttack` (`self.BPC_Attacks`) (make `/Game/Attacks/S_AttackInfo` AttackTarget "/Game/Enemies/Soseji2/Animation/Montage_Sword_Jump_Attack.Montage_Sword_Jump_Attack" (make `/Game/DamageSystem/S_DamageInfo` _new_atk "NewEnumerator1" "NewEnumerator0" false true true))))

(event `SpinningAttack`
  (params (AttackTarget :type "Actor Object Reference"))
  ;[1 1 1] Attacks
  (bind _new_atk (`self.ATK` 2.0))
  (`/Game/Attacks/BPC_Attacks.SpinningMeleeAttack` (`self.BPC_Attacks`) (make `/Game/Attacks/S_AttackInfo` AttackTarget "/Game/Enemies/Soseji2/Animation/Montage_Sword_SpinningAttack.Montage_Sword_SpinningAttack" (make `/Game/DamageSystem/S_DamageInfo` _new_atk "NewEnumerator1" "NewEnumerator0" false true))))

(event `self.Blocked`
  (`|PlayMontage` (`self.Mesh`) "/Game/Enemies/Soseji2/Animation/Montage_Sword_Block.Montage_Sword_Block"
    (:`OnCompleted`
      _)
    (:`OnInterrupted`
      _))
  (`self.EndBlock`))

(event `/Game/Enemies/AI/BPI_EnemyAI.EquipWeapon`
  ;[1 1 1] Equip/Unequip weapon
  (bind _notifyname (`|PlayMontage` (`self.Mesh`) "/Game/Enemies/Soseji2/Animation/Unsheath_Soseji.Unsheath_Soseji")
    (:`OnCompleted`
      (`self.OnWeaponEquipped`))
    (:`OnNotifyBegin`
      (switch `name` _notifyname
        (:`HoldSword`
          (bind _returnvalue (`|SpawnActorFromClass` "/Game/Weapons/BP_Weapon_Fork.BP_Weapon_Fork_C" (`self.GetTransform`) "Undefined" "MultiplyWithRoot" null null))
          (bind _output_get (set `self.WeaponActor` _returnvalue))
          (`self.K2_AttachToComponent` _output_get (`self.Mesh`) "hand_r_sword_socket" "SnapToTarget" "SnapToTarget" "SnapToTarget" true)
          (set `self.IsWieldingWeapon` true))))))

(event `/Game/Enemies/AI/BPI_EnemyAI.UnequipWeapon`
  ;[1 1 1] Equip/Unequip weapon
  (bind _notifyname (`|PlayMontage` (`self.Mesh`) "/Game/Enemies/Soseji2/Animation/Sheath_Soseji.Sheath_Soseji")
    (:`OnCompleted`
      (`self.OnWeaponUnequipped`))
    (:`OnNotifyBegin`
      (switch `name` _notifyname
        (:`DropSword`
          (`self.K2_DestroyActor` (`self.WeaponActor`))
          (set `self.IsWieldingWeapon` false))))))

(fn `ATK`
  (params (Base_ATK :type "Float (double-precision)"))
  (returns (New_ATK :type "Float (double-precision)"))
  (bind _ashensuu (cast `/Game/ThirdPerson/Blueprints/hensuu` (`GameplayStatics.GetGameInstance`)))
  (return (* (`/Game/ThirdPerson/Blueprints/hensuu.tuyosa` _ashensuu) Base_ATK)))

(fn `CalculateFutureActorLocation`
  (params (Actor :type "Actor Object Reference") (Time :type "Float (double-precision)" :default 1.0))
  (returns (Location :type "Vector Structure"))
  (return (+ (`self.K2_GetActorLocation` Actor) (* (* (`self.GetVelocity` Actor) (1.0 1.0 0.0)) Time))))

(fn `GetIdealRange`
  (returns (AttackRadius :type "Float (double-precision)") (DefendRadius :type "Float (double-precision)"))
  (return 200.0 400.0))

(fn `UserConstructionScript`
  (`parent.UserConstructionScript`)
  (set `self.MeshRotationBeforeSpin` (`SceneComponent.RelativeRotation` (`self.Mesh`))))