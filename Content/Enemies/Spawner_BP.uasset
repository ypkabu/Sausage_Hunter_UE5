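; Level spawner that fills its box with AI enemies and random items, and advances waves when enemies die.
; Spawns patrolling Ranged or Melee enemies up to the GameInstance quota on a timer quickening over time, retrying failed spawns.
; A rare Mage triggers a fire warning until all Mages die.
; Clearing enemies updates the wave and opens the next stage, boss or clear level; boss levels double Tuyosa, with separate Boss_Spawn logic.
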(event `DeathEnemy`
  (`KismetSystemLibrary.Delay` 1.0)
  (bind _outactors (`GameplayStatics.GetAllActorsOfClass` "/Game/Enemies/MageEnemy/BP_Enemy_Mage.BP_Enemy_Mage_C"))
  (if (== (`KismetArrayLibrary.Array_Length` _outactors) 0)
    (if (not (`self.IsFire?`))
      (`/Game/Widgets/FireMessage.FireDestroy` (`self.NewVar`))
      (set `self.IsFire?` true)
      (`AudioComponent.Stop` (`self.Sound`)))
    (bind _outactors_2 (`GameplayStatics.GetAllActorsWithTag` "enemy"))
    (if (== (`KismetArrayLibrary.Array_Length` _outactors_2) 0)
      (bind _ashensuu (cast `/Game/ThirdPerson/Blueprints/hensuu` (`GameplayStatics.GetGameInstance`)))
      (switch `/Game/ThirdPerson/Enum/Wave` (`/Game/ThirdPerson/Blueprints/hensuu.Wave` _ashensuu)
        (:`NewEnumerator0`
          (set `/Game/ThirdPerson/Blueprints/hensuu.Wave` "NewEnumerator1" _ashensuu)
          (bind _ashensuu_2 (cast `/Game/ThirdPerson/Blueprints/hensuu` (`GameplayStatics.GetGameInstance`) :!label _label))
          (set `/Game/ThirdPerson/Blueprints/hensuu.SpawnS2` (+ (`/Game/ThirdPerson/Blueprints/hensuu.SpawnS2` _ashensuu_2) (`KismetMathLibrary.RandomIntegerInRange` 0 1)) _ashensuu_2)
          (`GameplayStatics.OpenLevelBySoftObjectPtr` "/Game/ThirdPerson/Maps/Stage1.Stage1"))
        (:`NewEnumerator1`
          (set `/Game/ThirdPerson/Blueprints/hensuu.Wave` "NewEnumerator2" _ashensuu)
          (goto _label))
        (:`NewEnumerator2`
          (set `/Game/ThirdPerson/Blueprints/hensuu.Wave` "NewEnumerator3" _ashensuu)
          (`GameplayStatics.OpenLevelBySoftObjectPtr` (select `/Game/ThirdPerson/Enum/Stage` (`/Game/ThirdPerson/Blueprints/hensuu.Stage` _ashensuu) :`NewEnumerator0` "/Game/ThirdPerson/Maps/Boss1.Boss1" :`NewEnumerator1` "/Game/ThirdPerson/Maps/Boss2.Boss2" :`NewEnumerator2` "/Game/ThirdPerson/Maps/Stage3.Stage3" :!type "World Soft Object Reference")))
        (:`NewEnumerator3`
          (set `/Game/ThirdPerson/Blueprints/hensuu.CorDorM` "NewEnumerator0" _ashensuu)
          (`GameplayStatics.OpenLevelBySoftObjectPtr` "/Game/Title/Death_Crear.Death_Crear"))))))

(event `self.ReceiveBeginPlay`
  (`KismetSystemLibrary.Delay` 0.5)
  (bind _ashensuu (cast `/Game/ThirdPerson/Blueprints/hensuu` (`GameplayStatics.GetGameInstance`)))
  (set `/Game/ThirdPerson/Blueprints/hensuu.EnemyS` (`/Game/ThirdPerson/Blueprints/hensuu.SpawnS2` _ashensuu) _ashensuu)
  (`KismetSystemLibrary.Delay` 4.0)
  (`self.ItemSpawn`)
  (bind _returnvalue (`GameplayStatics.GetCurrentLevelName` true))
  (switch `string` _returnvalue
    (:`Stage1`
      (`self.Spawn` :!label _label_2)
      (`KismetSystemLibrary.Delay` 2.0)
      (bind _noenemy (`self.No Enemy Error`))
      (if _noenemy
        (`self.Spawn`)))
    (:`Stage2`
      (goto _label_2))
    (:`Stage3`
      (goto _label_2))
    (:`Boss1`
      (set `/Game/ThirdPerson/Blueprints/hensuu.tuyosa` (* (`/Game/ThirdPerson/Blueprints/hensuu.tuyosa` _ashensuu) 2.0) _ashensuu :!label _label_3))
    (:`Boss2`
      (goto _label_3))
    (:`Boss3`
      (goto _label_3))))

(event `Spawn`
  (bind _enemytype (`self.EnemyType`))
  (bind (_origin _boxextent) (`KismetSystemLibrary.GetComponentBounds` (`self.Box`)))
  (bind _ashensuu (cast `/Game/ThirdPerson/Blueprints/hensuu` (`GameplayStatics.GetGameInstance`)))
  (if (< (`self.EnemyPiace`) (`/Game/ThirdPerson/Blueprints/hensuu.SpawnS2` _ashensuu)) :!label _label_4
    (if (< (`KismetMathLibrary.RandomIntegerInRange` 0 100) 5)
      (if (`self.IsFire?`)
        (set `self.IsFire?` false)
        (bind _returnvalue (`|CreateWidget` "/Game/Widgets/FireMessage.FireMessage_C"))
        (`UserWidget.AddToViewport` _returnvalue 0)
        (set `self.NewVar` _returnvalue)
        (bind _returnvalue_2 (`GameplayStatics.SpawnSound2D` "/Game/sound/SE/arato_Cue.arato_Cue" 1.0 1.0 0.0 null))
        (set `self.Sound` _returnvalue_2))
      (set `self.EnemyType` "NewEnumerator2")
      (else
        (set `self.EnemyType` (select `int` (`KismetMathLibrary.RandomIntegerInRange` 0 1) :`0` "NewEnumerator0" :`1` "NewEnumerator1" :`2` "NewEnumerator2" :!type "/Game/Enemies/AI/Enums/E_EnemyType Enum"))))
    (bind _returnvalue_3 (`AIBlueprintHelperLibrary.SpawnAIFromClass` (select `/Game/Enemies/AI/Enums/E_EnemyType` _enemytype :`NewEnumerator0` "/Game/Enemies/BP_Enemy_Ranged.BP_Enemy_Ranged_C" :`NewEnumerator1` "/Game/Enemies/MeleeEnemy/BP_Enemy_Melee.BP_Enemy_Melee_C" :`NewEnumerator2` "/Game/Enemies/MageEnemy/BP_Enemy_Mage.BP_Enemy_Mage_C" :!type "Pawn Class Reference") (select `/Game/Enemies/AI/Enums/E_EnemyType` _enemytype :`NewEnumerator0` "/Game/Enemies/AI/BehaviorTrees/BT_Enemy_Ranged.BT_Enemy_Ranged" :`NewEnumerator1` "/Game/Enemies/AI/BehaviorTrees/BT_Enemy_Melee.BT_Enemy_Melee" :`NewEnumerator2` "/Game/Enemies/AI/BehaviorTrees/BT_Enemy_Mage.BT_Enemy_Mage" :!type "BehaviorTree Object Reference") (`KismetMathLibrary.RandomPointInBoundingBox` _origin _boxextent) (struct) false null))
    (`/Engine/EditorBlueprintResources/StandardMacros.IncrementFloat` (`self.EnemyPiace`)
      (:`  `
        (switch `/Game/Enemies/AI/Enums/E_EnemyType` (`self.EnemyType`)
          (:`NewEnumerator0`
            (bind _asbp_enemy_ranged (cast `/Game/Enemies/BP_Enemy_Ranged` _returnvalue_3))
            (set `/Game/Enemies/BP_Enemy_Base.PatrolRoute` (`self.patrolrote`) _asbp_enemy_ranged))
          (:`NewEnumerator1`
            (bind _asbp_enemy_melee (cast `/Game/Enemies/MeleeEnemy/BP_Enemy_Melee` _returnvalue_3))
            (set `/Game/Enemies/BP_Enemy_Base.PatrolRoute` (`self.patrolrote`) _asbp_enemy_melee))
          (:`NewEnumerator2`
            (bind _asbp_enemy_mage (cast `/Game/Enemies/MageEnemy/BP_Enemy_Mage` _returnvalue_3))
            (set `/Game/Enemies/BP_Enemy_Base.PatrolRoute` (`self.patrolrote`) _asbp_enemy_mage)))
        (bind _noenemy (`self.No Enemy Error`))
        (if _noenemy
          (goto _label_4)
          (else
            (`KismetSystemLibrary.K2_SetTimerDelegate` (delegate `Spawn`) (`KismetMathLibrary.Lerp` 1.0 0.01 (`self.Spawn Rate Ratio`)) true)))))
    (else
      (`KismetSystemLibrary.PrintString` "compleat"))))

(event `ItemSpawn`
  (bind (_origin _boxextent) (`KismetSystemLibrary.GetComponentBounds` (`self.Box`)))
  (`|SpawnActorFromClass` (select `int` (`KismetMathLibrary.RandomIntegerInRange` 0 3) :`0` "/Game/Inventory/item/ItemKechap.ItemKechap_C" :`1` "/Game/Inventory/item/ItemMastard.ItemMastard_C" :`2` "/Game/Inventory/item/ItemPikurus.ItemPikurus_C" :`3` "/Game/Inventory/item/ItemOnion.ItemOnion_C" :!type "Actor Class Reference") (`KismetMathLibrary.Conv_VectorToTransform` (`KismetMathLibrary.RandomPointInBoundingBox` _origin _boxextent)) "Undefined" "MultiplyWithRoot" null null)
  (`KismetSystemLibrary.K2_SetTimerDelegate` (delegate `ItemSpawn`) (`KismetMathLibrary.RandomFloatInRange` 4.0 10.0)))

(event `self.ReceiveTick`
  (params (DeltaSeconds :type "Float (single-precision)"))
  (bind _output_get (set `self.Elapsed Time` (+ (`GameplayStatics.GetWorldDeltaSeconds`) (`self.Elapsed Time`))))
  (set `self.Spawn Rate Ratio` (`KismetMathLibrary.MapRangeClamped` _output_get 0.0 20.0)))

(event `Boss_Spawn`
  (bind _enemytype (`self.EnemyType`))
  (bind (_origin _boxextent) (`KismetSystemLibrary.GetComponentBounds` (`self.Box`)))
  (if (< (`KismetMathLibrary.RandomIntegerInRange` 0 100) 5)
    (if (`self.IsFire?`)
      (set `self.IsFire?` false)
      (bind _returnvalue (`|CreateWidget` "/Game/Widgets/FireMessage.FireMessage_C"))
      (`UserWidget.AddToViewport` _returnvalue 0)
      (set `self.NewVar` _returnvalue))
    (set `self.EnemyType` "NewEnumerator2")
    (else
      (set `self.EnemyType` "NewEnumerator1")))
  (bind _returnvalue_2 (`AIBlueprintHelperLibrary.SpawnAIFromClass` (select `/Game/Enemies/AI/Enums/E_EnemyType` _enemytype :`NewEnumerator0` "/Game/Enemies/BP_Enemy_Ranged.BP_Enemy_Ranged_C" :`NewEnumerator1` "/Game/Enemies/MeleeEnemy/BP_Enemy_Melee.BP_Enemy_Melee_C" :`NewEnumerator2` "/Game/Enemies/MageEnemy/BP_Enemy_Mage.BP_Enemy_Mage_C" :!type "Pawn Class Reference") (select `/Game/Enemies/AI/Enums/E_EnemyType` _enemytype :`NewEnumerator0` "/Game/Enemies/AI/BehaviorTrees/BT_Enemy_Ranged.BT_Enemy_Ranged" :`NewEnumerator1` "/Game/Enemies/AI/BehaviorTrees/BT_Enemy_Melee.BT_Enemy_Melee" :`NewEnumerator2` "/Game/Enemies/AI/BehaviorTrees/BT_Enemy_Mage.BT_Enemy_Mage" :!type "BehaviorTree Object Reference") (`KismetMathLibrary.RandomPointInBoundingBox` _origin _boxextent) (struct) false null))
  (switch `/Game/Enemies/AI/Enums/E_EnemyType` (`self.EnemyType`)
    (:`NewEnumerator0`
      (bind _asbp_enemy_ranged (cast `/Game/Enemies/BP_Enemy_Ranged` _returnvalue_2))
      (set `/Game/Enemies/BP_Enemy_Base.PatrolRoute` (`self.patrolrote`) _asbp_enemy_ranged))
    (:`NewEnumerator1`
      (bind _asbp_enemy_melee (cast `/Game/Enemies/MeleeEnemy/BP_Enemy_Melee` _returnvalue_2))
      (set `/Game/Enemies/BP_Enemy_Base.PatrolRoute` (`self.patrolrote`) _asbp_enemy_melee))
    (:`NewEnumerator2`
      (bind _asbp_enemy_mage (cast `/Game/Enemies/MageEnemy/BP_Enemy_Mage` _returnvalue_2))
      (set `/Game/Enemies/BP_Enemy_Base.PatrolRoute` (`self.patrolrote`) _asbp_enemy_mage))))

(fn `No Enemy Error`
  (returns (NoEnemy :type Boolean))
  (bind _outactors (`GameplayStatics.GetAllActorsWithTag` "Enemy"))
  (bind _output_get (set `self.Out Actors` _outactors))
  (if (== (`KismetArrayLibrary.Array_Length` _output_get) (`self.EnemyPiace`))
    (return false)
    (else
      (`/Engine/EditorBlueprintResources/StandardMacros.DecrementFloat` (`self.EnemyPiace`)
        (:`  `
          (`KismetSystemLibrary.PrintString` "Error")
          (return true))))))

(fn `UserConstructionScript`)