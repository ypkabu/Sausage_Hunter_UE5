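; BP_effect is an environment actor that shows a Niagara heat distortion effect once the player's score reaches one.
; Tick casts the player character to BP_Player and checks ScoreP.
; At that threshold it spawns NS_HeatDistortion, scaled up, at the Cube's world location, storing it in Heat and respawning only when that reference is invalid.
; A separate SpawnEffect function makes an attached spawn with no template set and is not called here.
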(event `self.ReceiveTick`
  (params (DeltaSeconds :type "Float (single-precision)"))
  (bind _asbp_player (cast `/Game/Player/BP_Player` (`GameplayStatics.GetPlayerCharacter` 0)))
  (if (>= (`/Game/Player/BP_Player.ScoreP` _asbp_player) 1.0)
    (`self.Heat`
      (:`then`)
      (:`else`
        (bind _returnvalue (`NiagaraFunctionLibrary.SpawnSystemAtLocation` "/Game/environment/NS_HeatDistortion.NS_HeatDistortion" (`SceneComponent.K2_GetComponentLocation` (`self.Cube`)) (struct) (5.0 5.0 5.0)))
        (set `self.Heat` _returnvalue)))))

(fn `Spawn effect`
  (returns (ReturnValue :type "NiagaraComponent Object Reference"))
  (bind _returnvalue (`NiagaraFunctionLibrary.SpawnSystemAttached` null null "None" (0.0 0.0 0.0) (struct) "KeepRelativeOffset"))
  (return _returnvalue))

(fn `UserConstructionScript`)